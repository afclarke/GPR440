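; BP_FoodPellet is a food pellet actor that drifts with the tank's flow field, moves vertically and expires.
; Each tick, FlowFall samples PTankFlowField from UtilGameMode at the pellet's location.
; It combines the horizontal flow, scaled by FlowSpeed, with FallSpeed on Z into a swept, frame-rate-independent offset.
; Expire then counts down Lifetime and destroys the actor when it runs out.
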(event `self.ReceiveTick`
  (params (DeltaSeconds :type "Float (single-precision)"))
  (`self.FlowFall` DeltaSeconds)
  (`self.Expire` DeltaSeconds))

(fn `Expire`
  (params (Deltatime :type "Float (double-precision)"))
  (bind _output_get (set `self.Lifetime` (- (`self.Lifetime`) Deltatime)))
  (if (<= _output_get 0.0)
    (`self.K2_DestroyActor`)))

(fn `FlowFall`
  (params (DeltaTime :type "Float (double-precision)"))
  (bind _asutil_game_mode (cast `UtilGameMode` (`GameplayStatics.GetGameMode`)))
  (bind _returnvalue (`TankFlowField.GetFlowAtLoc` (`UtilGameMode.pTankFlowField` _asutil_game_mode) (`self.K2_GetActorLocation`)))
  (bind (_returnvalue_x _returnvalue_y) (`KismetMathLibrary.BreakVector2D` (* _returnvalue (`self.FlowSpeed`))))
  (`self.K2_AddActorWorldOffset` (* (`KismetMathLibrary.MakeVector` _returnvalue_x _returnvalue_y (`self.FallSpeed`)) DeltaTime) true))

(fn `UserConstructionScript`)
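; Crab agent for a utility-based AI system, implementing the crab's eat and attack actions.
; BindAct binds each incoming action to its crab handler by action type.
; Eating calls the Eat function, while attacking queries the game mode's quadtree for the closest FISH-tagged actor within attack range.
; A fish found this way is destroyed and the crab's Hunger is set to MaxHunger.
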(event `self.BindAct`
  (params (pAction :type "UtilAction Object Reference"))
  (switch `EUtilActionType` (`UtilAction.mActionType` pAction)
    (:`EAT`
      (add `UtilAction.mAct` pAction (`|CreateDelegate` :!event `CrabEat`)))
    (:`ATTACK`
      (add `UtilAction.mAct` pAction (`|CreateDelegate` :!event `CrabAttack`)))))

(event `CrabEat`
  (params (DeltaTime :type "Float (double-precision)"))
  (`self.Eat`))

(event `CrabAttack`
  (params (DeltaTime :type "Float (double-precision)"))
  (bind _asutil_game_mode (cast `UtilGameMode` (`GameplayStatics.GetGameMode`)))
  (bind _returnvalue (`QuadTree.FindClosestInRadius` (`UtilGameMode.mpQuadTree` _asutil_game_mode) self (`self.AttackRadiusSqr`) "FISH"))
  (`/Engine/EditorBlueprintResources/StandardMacros.IsValid` _returnvalue
    (:`Is Valid`
      (`self.K2_DestroyActor` _returnvalue)
      (set `self.Hunger` (`self.MaxHunger`)))))

(fn `UserConstructionScript`
  (`parent.UserConstructionScript`))
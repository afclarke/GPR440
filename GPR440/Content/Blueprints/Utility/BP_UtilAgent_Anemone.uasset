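; BP_UtilAgent_Anemone is a utility agent for an anemone that can hide or extend by changing its size.
; BindAct matches each action's type, HIDE or EXTEND, and binds an event to that action.
; The Hide and Extend acts lerp actor scale from its current value toward HidingScale or ExtendedScale by DeltaTime times ScaleSpeed, giving an eased transition.
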(event `self.ReceiveTick`
  (params (DeltaSeconds :type "Float (single-precision)"))
  (`parent.ReceiveTick` DeltaSeconds))

(event `self.BindAct`
  (params (pAction :type "UtilAction Object Reference"))
  (switch `EUtilActionType` (`UtilAction.mActionType` pAction)
    (:`HIDE`
      (add `UtilAction.mAct` pAction (`|CreateDelegate` :!event `Hide`)))
    (:`EXTEND`
      (add `UtilAction.mAct` pAction (`|CreateDelegate` :!event `Extend`)))))

(event `Hide`
  (params (DeltaTime :type "Float (double-precision)"))
  (`self.SetActorScale3D` (`KismetMathLibrary.VLerp` (`self.GetActorScale3D`) (`self.HidingScale`) (* DeltaTime (`self.ScaleSpeed`)))))

(event `Extend`
  (params (DeltaTime :type "Float (double-precision)"))
  (`self.SetActorScale3D` (`KismetMathLibrary.VLerp` (`self.GetActorScale3D`) (`self.ExtendedScale`) (* DeltaTime (`self.ScaleSpeed`)))))

(fn `UserConstructionScript`)
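; BP_UtilConsideration_ProximityAnemone is a utility AI consideration that scores how close an agent is to the nearest anemone.
; Perceive queries the game mode's quadtree for ANEMONE-tagged actors within MaxDistSqr and keeps the smallest squared distance.
; It returns that distance divided by MaxDistSqr, so the score nears 0 beside an anemone and is 1 when none is in range.
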(fn `perceive`
  (params (pAgent :type "UtilAgent Object Reference") (pGameMode :type "UtilGameMode Object Reference"))
  (returns (ReturnValue :type "Float (double-precision)"))
  (locals (ClosestDistSqr :type "Float (double-precision)"))
  (bind _returnvalue (`QuadTree.QuerySqrRadius` (`UtilGameMode.mpQuadTree` pGameMode) pAgent (`self.MaxDistSqr`) "ANEMONE"))
  (set `local.ClosestDistSqr` (`self.MaxDistSqr`))
  (for _array_element _returnvalue
    (bind _returnvalue_2 (`KismetMathLibrary.VSizeSquared` (- (`Actor.K2_GetActorLocation` _array_element) (`Actor.K2_GetActorLocation` pAgent))))
    (if (>= (`local.ClosestDistSqr`) _returnvalue_2)
      (set `local.ClosestDistSqr` _returnvalue_2)))
  (return (/ (`local.ClosestDistSqr`) (`self.MaxDistSqr`))))
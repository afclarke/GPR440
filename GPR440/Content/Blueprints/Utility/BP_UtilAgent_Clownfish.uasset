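; BP_UtilAgent_Clownfish is a clownfish utility-AI agent that moves with the tank's water flow and can flock.
; Each Tick samples the game mode's flow field at its location and adds that as scaled movement input.
; Act dispatches on action type: Flock feeds weighted separation, alignment and cohesion among tagged mates into the floating pawn movement.
; Hide and Explore are empty stubs that still report success.
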(event `self.ReceiveTick`
  (params (DeltaSeconds :type "Float (single-precision)"))
  (`parent.ReceiveTick` DeltaSeconds)
  (bind _asutil_game_mode (cast `UtilGameMode` (`GameplayStatics.GetGameMode`)))
  (bind _returnvalue (`TankFlowField.GetFlowAtLoc` (`UtilGameMode.pTankFlowField` _asutil_game_mode) (`self.K2_GetActorLocation`)))
  (bind (_returnvalue_x _returnvalue_y) (`KismetMathLibrary.BreakVector2D` (* _returnvalue (`self.FlowSpeed`))))
  (`self.AddMovementInput` (`KismetMathLibrary.MakeVector` _returnvalue_x _returnvalue_y)))

(fn `Act`
  (params (actionType :type "EUtilActionType Enum" :default "INVALID"))
  (returns (ReturnValue :type Boolean))
  (switch `EUtilActionType` actionType
    (:`INVALID`
      (return false))
    (:`HIDE`
      (`self.Hide`)
      (return true))
    (:`EXPLORE`
      (`self.Explore`)
      (return true))
    (:`FLOCK`
      (bind _returnvalue (`self.Flock` 10000.0 50000.0 50000.0 2.0 0.4 0.2 (`self.FlockMateTag`)))
      (bind (_returnvalue_x _returnvalue_y) (`KismetMathLibrary.BreakVector2D` (* _returnvalue (`self.FlockSpeed`))))
      (`PawnMovementComponent.AddInputVector` (`self.FloatingPawnMovement`) (`KismetMathLibrary.MakeVector` _returnvalue_x _returnvalue_y) false))))

(fn `Explore`)

(fn `Hide`)

(fn `UserConstructionScript`
  (`parent.UserConstructionScript`))
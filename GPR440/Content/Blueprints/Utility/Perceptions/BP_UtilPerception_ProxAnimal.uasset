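; Utility AI perception that scores an agent's proximity to the nearest actor tagged as an animal.
; Perceive queries the game mode's quadtree for the closest animal within a squared radius.
; It returns the squared distance divided by that squared radius, so closer animals give values nearer zero.
; When no animal is found it returns one.
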(fn `perceive`
  (params (pAgent :type "UtilAgent Object Reference") (pGameMode :type "UtilGameMode Object Reference"))
  (returns (ReturnValue :type "Float (double-precision)"))
  (bind _returnvalue (`QuadTree.FindClosestInRadius` (`UtilGameMode.mpQuadTree` pGameMode) pAgent (`self.RadiusSqr`) "ANIMAL"))
  (`/Engine/EditorBlueprintResources/StandardMacros.IsValid` _returnvalue
    (:`Is Valid`
      (return (/ (`KismetMathLibrary.Vector_DistanceSquared` (`Actor.K2_GetActorLocation` _returnvalue) (`Actor.K2_GetActorLocation` pAgent)) (`self.RadiusSqr`))))
    (:`Is Not Valid`
      (return 1.0))))
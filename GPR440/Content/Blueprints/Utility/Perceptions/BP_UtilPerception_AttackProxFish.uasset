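; Utility AI perception that scores how close the nearest fish is within the agent's attack radius.
; Perceive queries the game mode's quadtree for the closest FISH-tagged actor inside the agent's squared attack radius.
; It returns that squared distance divided by the squared radius, so nearer fish give lower values, and 1.0 when none is found.
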(fn `perceive`
  (params (pAgent :type "UtilAgent Object Reference") (pGameMode :type "UtilGameMode Object Reference"))
  (returns (ReturnValue :type "Float (double-precision)"))
  (bind _asbp_util_agent (cast `/Game/Blueprints/Utility/BP_UtilAgent` pAgent))
  (bind _returnvalue (`QuadTree.FindClosestInRadius` (`UtilGameMode.mpQuadTree` pGameMode) _asbp_util_agent (`/Game/Blueprints/Utility/BP_UtilAgent.AttackRadiusSqr` _asbp_util_agent) "FISH"))
  (`/Engine/EditorBlueprintResources/StandardMacros.IsValid` _returnvalue
    (:`Is Valid`
      (return (/ (`KismetMathLibrary.Vector_DistanceSquared` (`Actor.K2_GetActorLocation` _returnvalue) (`Actor.K2_GetActorLocation` _asbp_util_agent)) (`/Game/Blueprints/Utility/BP_UtilAgent.AttackRadiusSqr` _asbp_util_agent))))
    (:`Is Not Valid`
      (return 1.0))))
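; Cardinal fish utility AI agent that supplies the fish's flocking and eating behaviours.
; BindAct switches on each action's type to bind an event for the flock and eat actions.
; Flocking blends separation, alignment and cohesion among CARDINAL-tagged agents using squared radii, then feeds only X and Y into movement input scaled by FlockSpeed.
; Eating simply calls Eat, and the default lifecycle events are unused.
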(event `self.BindAct`
  (params (pAction :type "UtilAction Object Reference"))
  (switch `EUtilActionType` (`UtilAction.mActionType` pAction)
    (:`FLOCK`
      (add `UtilAction.mAct` pAction (`|CreateDelegate` :!event `FlockCardinal`)))
    (:`EAT`
      (add `UtilAction.mAct` pAction (`|CreateDelegate` :!event `EatCardinal`)))))

(event `FlockCardinal`
  (params (DeltaTime :type "Float (double-precision)"))
  (bind _returnvalue (`self.Flock` 20000.0 80000.0 1000000.0 4.0 2.0 2.0 "CARDINAL"))
  (`self.AddMovementInput` (`KismetMathLibrary.MakeVector` (`KismetMathLibrary.BreakVector2D` _returnvalue) (`.Y` (`KismetMathLibrary.BreakVector2D` _returnvalue))) (`self.FlockSpeed`)))

(event `EatCardinal`
  (params (DeltaTime :type "Float (double-precision)"))
  (`self.Eat`))

(fn `UserConstructionScript`
  (`parent.UserConstructionScript`))
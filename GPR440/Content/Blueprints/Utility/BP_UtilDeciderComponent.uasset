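; Utility decider component that displays its actions through an on-screen WBP_Utility widget.
; On BeginPlay it creates the widget and adds it to the viewport, then copies MActionObjs into the widget's Actions every Tick.
; Enable and disable functions toggle the widget's Paint flag, while the decision logic itself is not in these graphs.
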(event `self.ReceiveBeginPlay`
  (bind _returnvalue (`|CreateWidget` "/Game/Blueprints/Utility/WBP_Utility.WBP_Utility_C"))
  (bind _output_get (set `self.UtilityWidget` _returnvalue))
  (`UserWidget.AddToViewport` _output_get 0))

(event `self.ReceiveTick`
  (params (DeltaSeconds :type "Float (single-precision)"))
  (set `/Game/Blueprints/Utility/WBP_Utility.Actions` (`self.mActionObjs`) (`self.UtilityWidget`)))

(fn `DisableUtilityWidget`
  (set `/Game/Blueprints/Utility/WBP_Utility.Paint` false (`self.UtilityWidget`)))

(fn `EnableUtilityWidget`
  (set `/Game/Blueprints/Utility/WBP_Utility.Paint` true (`self.UtilityWidget`)))
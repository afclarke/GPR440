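; BP_Player is a mouse-driven player Blueprint for inspecting utility agents and dropping food pellets.
; Right click hides the current agent's utility widget, then line-traces from the cursor to select a BP_UtilAgent and show its widget.
; Left click spawns a scaled-down BP_FoodPellet along the deprojected cursor ray, using camera height minus FeedZ as the distance.
; BeginPlay enables the mouse cursor.
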(event `self.ReceiveBeginPlay`
  (set `PlayerController.bShowMouseCursor` true (`GameplayStatics.GetPlayerController` 0)))

(event `Key|RightMouseButton`
  (params (Key :type "Key Structure"))
  (bind _activeselectedagent (`self.ActiveSelectedAgent`))
  (bind (_worldlocation _worlddirection) (`PlayerController.DeprojectMousePositionToWorld` (`GameplayStatics.GetPlayerController` 0)))
  (:`Pressed`
    (`/Engine/EditorBlueprintResources/StandardMacros.IsValid` _activeselectedagent
      (:`Is Valid`
        (`/Game/Blueprints/Utility/BP_UtilAgent.DisableUtilityWidget` _activeselectedagent))
      (:`Is Not Valid`
        _))
    (bind (_outhit _returnvalue) (`KismetSystemLibrary.LineTraceSingle` _worldlocation (+ _worldlocation (* _worlddirection (`self.LineTraceLength`))) "TraceTypeQuery1"))
    (if _returnvalue
      (bind _asbp_util_agent (cast `/Game/Blueprints/Utility/BP_UtilAgent` (`.HitActor` (`GameplayStatics.BreakHitResult` _outhit))))
      (bind _output_get (set `self.ActiveSelectedAgent` _asbp_util_agent))
      (`/Game/Blueprints/Utility/BP_UtilAgent.EnableUtilityWidget` _output_get))))

(event `Key|LeftMouseButton`
  (params (Key :type "Key Structure"))
  (bind (_worldlocation _worlddirection) (`PlayerController.DeprojectMousePositionToWorld` (`GameplayStatics.GetPlayerController` 0)))
  (:`Pressed`
    (`|SpawnActorFromClass` "/Game/Blueprints/BP_FoodPellet.BP_FoodPellet_C" (`KismetMathLibrary.MakeTransform` (+ _worldlocation (* _worlddirection (- (.z _worldlocation) (`self.FeedZ`)))) (struct) (0.4 0.4 0.4)) "AlwaysSpawn" "OverrideRootScale" null null)))

(fn `UserConstructionScript`)